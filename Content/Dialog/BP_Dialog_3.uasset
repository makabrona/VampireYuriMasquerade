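; Dialog actor that presents a two-choice question, with the top answer treated as correct and the bottom as wrong.
; On BeginPlay both answers and their outlines are hidden, then the answers appear after a short delay.
; Cursor hover toggles each answer's outline while AnswersVisible is set.
; A click hides both answers and prints the verdict, though either choice sets CorrectAnswer to true.
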(event OnClicked(TopAnswer)
  (params (TouchedComponent :type Primitive%20Component%20Object%20Reference) (ButtonPressed :type Key%20Structure))
  (if (Variables|Default|GetAnswers%20Visible)
    (Variables|Default|SetCorrectAnswer true)
    (Rendering|SetVisibility (Variables|Default|GetTopAnswer) false false)
    (Rendering|SetVisibility (Variables|Default|GetBottom%20answer) false false)
    (Variables|Default|SetAnswers%20Visible false)
    (Rendering|SetVisibility (Variables|Default|GetOutlineTop) false false)
    (Development|PrintString "Yay it is correct!!!")))

(event OnClicked(Bottomanswer)
  (params (TouchedComponent :type Primitive%20Component%20Object%20Reference) (ButtonPressed :type Key%20Structure))
  (if (Variables|Default|GetAnswers%20Visible)
    (Variables|Default|SetCorrectAnswer true)
    (Rendering|SetVisibility (Variables|Default|GetBottom%20answer) false false)
    (Rendering|SetVisibility (Variables|Default|GetTopAnswer) false false)
    (Variables|Default|SetAnswers%20Visible false)
    (Rendering|SetVisibility (Variables|Default|GetOutlineBottom) false false)
    (Development|PrintString "NOOOO it is wrong!!!")))

(event OnBeginCursorOver(TopAnswer)
  (params (TouchedComponent :type Primitive%20Component%20Object%20Reference))
  ;[0.15 0.15 0.15 0.5] Hovering over top answer
  (if (Variables|Default|GetAnswers%20Visible)
    (Rendering|SetVisibility (Variables|Default|GetOutlineTop) true false)))

(event OnEndCursorOver(TopAnswer)
  (params (TouchedComponent :type Primitive%20Component%20Object%20Reference))
  ;[0.15 0.15 0.15 0.5] Hovering over top answer
  (if (Variables|Default|GetAnswers%20Visible)
    (Rendering|SetVisibility (Variables|Default|GetOutlineTop) false false)))

(event OnBeginCursorOver(Bottomanswer)
  (params (TouchedComponent :type Primitive%20Component%20Object%20Reference))
  ;[0.15 0.15 0.15 0.5] Hovering over bottom answer
  (if (Variables|Default|GetAnswers%20Visible)
    (Rendering|SetVisibility (Variables|Default|GetOutlineBottom) true false)))

(event OnEndCursorOver(Bottomanswer)
  (params (TouchedComponent :type Primitive%20Component%20Object%20Reference))
  ;[0.15 0.15 0.15 0.5] Hovering over bottom answer
  (if (Variables|Default|GetAnswers%20Visible)
    (Rendering|SetVisibility (Variables|Default|GetOutlineBottom) false false)))

(event EventBeginPlay
  (Rendering|SetVisibility (Variables|Default|GetTopAnswer) false false)
  (Rendering|SetVisibility (Variables|Default|GetBottom%20answer) false false)
  (Rendering|SetVisibility (Variables|Default|GetOutlineTop) false false)
  (Rendering|SetVisibility (Variables|Default|GetOutlineBottom) false false)
  (Variables|Default|SetAnswers%20Visible false)
  (Utilities|FlowControl|Delay 2.0)
  (Rendering|SetVisibility (Variables|Default|GetTopAnswer) true false)
  (Rendering|SetVisibility (Variables|Default|GetBottom%20answer) true false)
  (Variables|Default|SetAnswers%20Visible true))

(fn ConstructionScript)