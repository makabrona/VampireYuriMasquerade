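; BPC_TitleState is a title-state Blueprint that is mostly a stub, with debug output for a finished-state event.
; Its OnStateFinished_Event handler binds itself to OnStateFinished, then prints the received state outcome enum on screen.
; BeginPlay, overlap and Tick are disabled default nodes, and the construction script only calls its parent.
; Nothing in this graph calls the handler or makes the initial binding.
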(event Custom|OnStateFinished_Event
  (params (EnumStateOutcome :type E_StateOutcome%20Enum :default "NewEnumerator0"))
  (EventDispatchers|BindEventtoOnStateFinished (delegate Custom|OnStateFinished_Event))
  (Development|PrintString (Utilities|String|EnumtoString EnumStateOutcome) true true "(R=0.000000,G=0.660000,B=1.000000,A=1.000000)" 1e+01))

(event EventBeginPlay
  (|CallParentFunction) ; This node is disabled and will not be called.\nDrag off pins to build functionality.
)

(event Collision|EventActorBeginOverlap
  (params (OtherActor :type Actor%20Object%20Reference))
  (|CallParentFunction OtherActor) ; This node is disabled and will not be called.\nDrag off pins to build functionality.
)

(event EventTick
  (params (DeltaSeconds :type Float%20%28single-precision%29))
  (|CallParentFunction DeltaSeconds) ; This node is disabled and will not be called.\nDrag off pins to build functionality.
)

(fn ConstructionScript
  (|CallParentFunction))