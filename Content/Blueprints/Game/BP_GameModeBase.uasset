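; Game mode Blueprint that shows the game's opening dialog and its end-of-game screens.
; BeginPlay creates the first-dialog widget and adds it to the viewport.
; The Lose and Win custom events each create and display their own screen, game over or win, without further game-state logic.
; An older main-menu startup chain remains in the graph but is disconnected and never runs.
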(event Custom|Event_Win
  (bind _returnvalue (UserInterface|CreateWidget "/Game/Widgets/GameOver/WBP_WinScreen.WBP_WinScreen_C"))
  (bind _output_get (Variables|Default|SetNewVar_0 _returnvalue))
  (UserInterface|Viewport|AddtoViewport _output_get 0))

(event Custom|Event_Lose
  (params (NewParam :type Boolean))
  (bind _returnvalue (UserInterface|CreateWidget "/Game/Widgets/GameOver/WBP_GameOverScreen.WBP_GameOverScreen_C"))
  (bind _output_get (Variables|Default|SetNewVar _returnvalue))
  (UserInterface|Viewport|AddtoViewport _output_get 0))

(event EventBeginPlay
  ;[0.15 0.15 0.15 0.5] Game start
  (bind _returnvalue (UserInterface|CreateWidget "/Game/Blueprints/HUD/WB_FirstDialog.WB_FirstDialog_C"))
  (bind _output_get (Variables|Default|SetWB_FirstDialog%20Ref _returnvalue))
  (UserInterface|Viewport|AddtoViewport _output_get 0))

(event EventTick
  (params (DeltaSeconds :type Float%20%28single-precision%29)))

(fn ConstructionScript)